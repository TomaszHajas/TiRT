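; Network node actor that holds a visible queue of packets bound for other nodes and releases them over time.
; Tick times each release with a selectable Poisson, On-Off, Exponential or Markov-modulated Poisson model, mostly randomized and tied to a maximum sending delay.
; AddRandomPacket spawns packets stacked above the node with random receiver and priority; RemovePacket sets one moving and restacks those behind it.
; GetRandomReceivers picks destinations from the other nodes.
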(event EventBeginPlay)

(event EventActorBeginOverlap
  (params (OtherActor :type Actor%20Object%20Reference)))

(event EventTick
  (params (DeltaSeconds :type Float%20%28single-precision%29))
  (switch int (Variables|Default|GetDistribution)
    (:0
      ;[1 1 1] Poisson
      (bind _output_get (Variables|Default|SetTimer (+ DeltaSeconds (Variables|Default|GetTimer))))
      (if (or (<= (* (Variables|Default|GetPoissonVariable) (Math|Random|RandomFloat)) (Class|KismetMathLibrary|Exp (* (Variables|Default|GetMaxSendingDelay) -0.5))) (>= _output_get (Variables|Default|GetMaxSendingDelay)))
        (Variables|Default|SetPoissonVariable 1.0)
        (Variables|Default|SetTimer 0.0)
        (CallFunction|RemovePacket (Utilities|Array|Get(acopy) (Variables|Default|GetQueue)))))
    (:1
      ;[1 1 1] On-Off
      (bind _output_get_2 (Variables|Default|SetTimer (+ DeltaSeconds (Variables|Default|GetTimer))))
      (if (>= _output_get_2 (Variables|Default|GetMaxSendingDelay))
        (Variables|Default|SetTimer 0.0)
        (CallFunction|RemovePacket (Utilities|Array|Get(acopy) (Variables|Default|GetQueue)))))
    (:2
      ;[1 1 1] Exponential
      (bind _output_get_3 (Variables|Default|SetTimer (+ DeltaSeconds (Variables|Default|GetTimer))))
      (if (>= (Class|KismetMathLibrary|Exp _output_get_3) (* (Class|KismetMathLibrary|Exp (Variables|Default|GetMaxSendingDelay)) (Math|Random|RandomFloat)))
        (Variables|Default|SetTimer 0.0)
        (CallFunction|RemovePacket (Utilities|Array|Get(acopy) (Variables|Default|GetQueue)))))
    (:3
      ;[1 1 1] Markov Modulated Poisson Process
      (Utilities|FlowControl|Sequence
        (:then_0
          (if (<= (* (Variables|Default|GetPoissonVariable) (Math|Random|RandomFloat)) (Class|KismetMathLibrary|Exp (* (Variables|Default|GetMaxSendingDelay) -0.5)))
            (Variables|Default|SetPoissonVariable 1.0)
            (Variables|Default|SetMarkovVariable (+ (Variables|Default|GetMarkovVariable) 0.05))))
        (:then_1
          (bind _output_get_4 (Variables|Default|SetTimer (+ DeltaSeconds (Variables|Default|GetTimer))))
          (if (or (>= _output_get_4 (Variables|Default|GetMaxSendingDelay)) (<= (Math|Random|RandomFloat) (Variables|Default|GetMarkovVariable)))
            (Variables|Default|SetPoissonVariable 1.0)
            (Variables|Default|SetMarkovVariable 0.0)
            (Variables|Default|SetTimer 0.0)
            (CallFunction|RemovePacket (Utilities|Array|Get(acopy) (Variables|Default|GetQueue)))))))))

(fn ConstructionScript)

(fn AddRandomPacket
  (bind _returnvalue (Transformation|GetActorTransform))
  (bind _receivers (Variables|Default|GetReceivers))
  (bind _returnvalue_2 (Game|SpawnActorfromClass "/Game/Blueprints/Packet.Packet_C" (Math|Transform|MakeTransform (Math|Vector|MakeVector (.x (.location _returnvalue)) (.y (.location _returnvalue)) (+ (.z (.location _returnvalue)) (Math|Conversions|ToFloat(Integer) (+ (* (+ (Utilities|Array|Length (Variables|Default|GetQueue)) 1) 6) 8)))) "0, 0, 0" "1,1,1") "Undefined" 0 0))
  (bind _output_get (Variables|/Game/Blueprints/Packet.Packet_C|SetSession%20id _returnvalue_2 (Math|Random|RandomInteger (Utilities|Array|Length _receivers))))
  (Variables|/Game/Blueprints/Packet.Packet_C|SetDST _returnvalue_2 (Utilities|Array|Get(acopy) _receivers _output_get))
  (Variables|/Game/Blueprints/Packet.Packet_C|SetSRC _returnvalue_2 self)
  (Variables|/Game/Blueprints/Packet.Packet_C|SetPacket%20id _returnvalue_2 (Variables|Default|GetLastNodeId))
  (Variables|/Game/Blueprints/Packet.Packet_C|SetPriority _returnvalue_2 (Math|Random|RandomInteger 10))
  (Variables|/Game/Blueprints/Packet.Packet_C|SetPayload _returnvalue_2 "Quick brown fox jumps over a lazy dog")
  (Default|SetColor _returnvalue_2)
  (Math|Integer|IncrementInt (Variables|Default|GetLastNodeId)
    (:%20%20
      (Utilities|Array|Add (Variables|Default|GetQueue) _returnvalue_2))))

(fn RemovePacket
  (params (Packet :type Packet%20Object%20Reference))
  (bind _returnvalue (Transformation|GetActorLocation))
  (LocalVariables|SetFoundPacket 0)
  (for (_array_element _array_index) (Variables|Default|GetQueue)
    (if (== _array_element Packet)
      (LocalVariables|SetFoundPacket _array_element)
      (Transformation|SetActorLocation _array_element (Transformation|GetActorLocation) false false)
      (Variables|/Game/Blueprints/Packet.Packet_C|SetIsMoving _array_element true)
      (elif (Utilities|IsValid (LocalVariables|GetFoundPacket))
        (Transformation|SetActorLocation _array_element (Math|Vector|MakeVector (.x _returnvalue) (.y _returnvalue) (+ (.z _returnvalue) (Math|Conversions|ToFloat(Integer) (+ (* _array_index 6) 8)))) false false))))
  (Utilities|Array|RemoveItem (Variables|Default|GetQueue) (LocalVariables|GetFoundPacket)))

(fn GetRandomReceivers
  (params (MinReceivers :type Integer) (MaxReceivers :type Integer))
  (bind _outactors (Actor|GetAllActorsOfClass "Node_C"))
  (Utilities|Array|RemoveItem _outactors self)
  (Utilities|Array|Shuffle _outactors)
  (for _index (range 1 (+ (Math|Random|RandomInteger (- MaxReceivers MinReceivers)) MinReceivers))
    (Utilities|Array|AddUnique (LocalVariables|GetResult) (Utilities|Array|Get(acopy) _outactors _index)))
  (return (LocalVariables|GetResult)))