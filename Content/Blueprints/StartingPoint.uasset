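; StartingPoint is an actor that builds a randomized network of Node actors around itself on BeginPlay and seeds it with packets.
; It retries random sphere traces until one is clear, then spawns a Node at a separately randomized position within 100 units per horizontal axis.
; It then shuffles all Nodes, assigns random receivers, sending delay and distribution settings, and adds random packets to each.
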(event `self.ReceiveBeginPlay`
  (bind (_returnvalue_x _returnvalue_y _returnvalue_z) (`KismetMathLibrary.BreakVector` (`self.K2_GetActorLocation`)))
  (bind _returnvalue (+ _returnvalue_x (- (* (`KismetMathLibrary.RandomFloat`) 200.0) 100.0)))
  (bind _returnvalue_2 (+ _returnvalue_y (- (* (`KismetMathLibrary.RandomFloat`) 200.0) 100.0)))
  (for _ (range 1 (+ (`self.NumberOfNodes`) 1))
    (bind _outhits (`KismetSystemLibrary.SphereTraceMulti_NEW` :`Start` (`KismetMathLibrary.MakeVector` _returnvalue _returnvalue_2 _returnvalue_z) :`End` (`KismetMathLibrary.MakeVector` _returnvalue _returnvalue_2 _returnvalue_z) :`Radius` 10.0 :`TraceChannel` "TraceTypeQuery1" :`DrawDebugType` "Persistent" :!label _label))
    (bind _returnvalue_3 (`KismetArrayLibrary.Array_Length` _outhits))
    (if (== _returnvalue_3 0)
      (bind _returnvalue_4 (`|SpawnActorFromClass` "/Game/Blueprints/Node.Node_C" (`KismetMathLibrary.MakeTransform` (`KismetMathLibrary.MakeVector` _returnvalue _returnvalue_2 _returnvalue_z)) "AdjustIfPossibleButAlwaysSpawn" "OverrideRootScale"))
      (`Pawn.SpawnDefaultController` (`Actor.Instigator` _returnvalue_4))
      (else
        (`KismetSystemLibrary.PrintString` (`KismetStringLibrary.Conv_IntToString` _returnvalue_3))
        (goto _label))))
  (bind _outactors (`GameplayStatics.GetAllActorsOfClass` "/Game/Blueprints/Node.Node_C"))
  (`KismetArrayLibrary.Array_Shuffle` _outactors)
  (for _array_element _outactors
    (bind _randomreceivers (`/Game/Blueprints/Node.GetRandomReceivers` _array_element (`self.MinReceivers`) (`self.MaxReceivers`)))
    (set `/Game/Blueprints/Node.Receivers` _randomreceivers _array_element)
    (set `/Game/Blueprints/Node.MaxSendingDelay` (`self.MaxSendingDelay`) _array_element)
    (set `/Game/Blueprints/Node.Distribution` (`self.Distribution`) _array_element))
  (for _array_element_2 _outactors
    (for _ (range 1 (+ (`self.PacketsInNodes`) 1))
      (`/Game/Blueprints/Node.AddRandomPacket` _array_element_2))))

(fn `UserConstructionScript`)