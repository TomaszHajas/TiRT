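; Packet actor that travels to a destination actor (DST), apparently visualizing traffic between network nodes.
; While IsMoving, Tick faces DST and steps one unit forward per frame, so speed depends on frame rate.
; On arrival it calls AddRandomPacket on DST and destroys itself, as it does if DST is invalid.
; BeginPlay tints the cylinder via a dynamic material, hashing SessionId into RGB and scaling Priority into alpha.
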(event `self.ReceiveBeginPlay`
  (`self.SetColor`))

(event `self.ReceiveTick`
  (params (DeltaSeconds :type "Float (single-precision)"))
  (bind _returnvalue (`self.K2_GetActorLocation`))
  (if (`self.IsMoving`)
    (if (`KismetSystemLibrary.IsValid` (`self.DST`))
      (if (== (`self.K2_GetActorLocation`) (`self.K2_GetActorLocation` (`self.DST`)) :`ErrorTolerance` 1.0)
        (`/Game/Blueprints/Node.AddRandomPacket` (`self.DST`))
        (`self.K2_DestroyActor`)
        (else
          (`self.SetActorRotation` (`KismetMathLibrary.FindLookAtRotation` _returnvalue (`self.K2_GetActorLocation` (`self.DST`))))
          (`self.K2_SetActorLocation` (+ _returnvalue (`self.GetActorForwardVector`)))))
      (else
        (`self.K2_DestroyActor`)))))

(fn `SetColor`
  (bind _session_id (`self.Session id`))
  (bind _returnvalue (`PrimitiveComponent.CreateDynamicMaterialInstance` (`self.Cylinder`) 0 "/Game/StarterContent/Materials/M_Basic_Floor.M_Basic_Floor"))
  (`MaterialInstanceDynamic.SetVectorParameterValue` _returnvalue "Color" (make `LinearColor` (mod (* (+ _session_id 3) 13.1) 1.0) (mod (* (+ _session_id 4) 12.2) 1.0) (mod (* (+ _session_id 5) 11.3) 1.0) (/ (+ (`KismetMathLibrary.Conv_IntToDouble` (`self.Priority`)) 1.0) 11.0))))

(fn `UserConstructionScript`)